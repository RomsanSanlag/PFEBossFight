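; BP_LightsOff_Alex is a level lighting controller that changes the intensity of two directional lights and a sky light when LightsOff is called.
; LightsOff prints a debug string and plays a timeline, which scales each light's intensity variable by the LightValue track on every update.
; BeginPlay casts BossRef to BP_BossCharacter but does nothing with the result, and nothing in this graph calls LightsOff.
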(event `self.ReceiveBeginPlay`
  (cast `/Game/StarterContent/Blueprints/BP_Boss/BP_BossCharacter` (`self.BossRef`)))

(event `LightsOff`
  (`KismetSystemLibrary.PrintString` "LightsOff")
  (bind (_direction _light_value) (`Timeline|Timeline`)
    (:`Update`
      (`LightComponent.SetIntensity` (`Light.LightComponent` (`self.DirLight1`)) (* (`self.LightIntensity1`) _light_value))
      (`LightComponent.SetIntensity` (`Light.LightComponent` (`self.DirLight2`)) (* (`self.LightIntensity2`) _light_value))
      (`SkyLightComponent.SetIntensity` (`SkyLight.LightComponent` (`self.SkyLight1`)) (* (`self.LightIntensity3`) _light_value)))))

(fn `UserConstructionScript`)