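; Blueprint that dims the level's directional light and skylight in stages during a boss encounter, ending in darkness.
; On BeginPlay it binds three lighting events (Lights50, Lights5, LightsOff) to BP_BossCharacter.
; The first two scale intensities through timelines and store the result as the new baseline, so the dimming compounds.
; LightsOff swaps in final post-process settings and sets both lights to zero, without a gradual fade.
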(event `self.ReceiveBeginPlay`
  (`|ExecutionSequence`
    (:`then_1`
      (bind _asbp_boss_character (cast `/Game/StarterContent/Blueprints/BP_Boss/BP_BossCharacter` (`self.BossRef`)))
      (add `/Game/StarterContent/Blueprints/BP_Boss/BP_BossCharacter.Lights50` _asbp_boss_character (delegate `Lights50`))
      (add `/Game/StarterContent/Blueprints/BP_Boss/BP_BossCharacter.Lights5` _asbp_boss_character (delegate `Lights5`))
      (add `/Game/StarterContent/Blueprints/BP_Boss/BP_BossCharacter.Lights0` _asbp_boss_character (delegate `LightsOff`)))))

(event `Lights50`
  (bind (_direction _light_value) (`Timeline|Timeline_50`)
    (:`Update`
      (bind _returnvalue (* (`self.DirLightIntensity`) _light_value))
      (`LightComponent.SetIntensity` (`Light.LightComponent` (`self.DirLight`)) _returnvalue)
      (bind _returnvalue_2 (* (`self.SkyLightIntensity`) _light_value))
      (`SkyLightComponent.SetIntensity` (`SkyLight.LightComponent` (`self.SkyLight`)) _returnvalue_2))
    (:`Finished`
      (set `self.DirLightIntensity` _returnvalue)
      (set `self.SkyLightIntensity` _returnvalue_2))))

(event `Lights5`
  (bind (_direction _light_value) (`Timeline|Timeline_5`)
    (:`Update`
      (bind _returnvalue (* (`self.DirLightIntensity`) _light_value))
      (`LightComponent.SetIntensity` (`Light.LightComponent` (`self.DirLight`)) _returnvalue)
      (bind _returnvalue_2 (* (`self.SkyLightIntensity`) _light_value))
      (`SkyLightComponent.SetIntensity` (`SkyLight.LightComponent` (`self.SkyLight`)) _returnvalue_2))
    (:`Finished`
      (set `self.DirLightIntensity` _returnvalue)
      (set `self.SkyLightIntensity` _returnvalue_2))))

(event `LightsOff`
  (set `PostProcessVolume.Settings` (`self.SettingsFinal`) (`self.PostProcessVolume`))
  (bind (_direction _timeline_0) (`Timeline|Timeline_0`)
    (:`Update`
      (`LightComponent.SetIntensity` (`Light.LightComponent` (`self.DirLight`)) 0.0)
      (`SkyLightComponent.SetIntensity` (`SkyLight.LightComponent` (`self.SkyLight`)) 0.0))))

(fn `UserConstructionScript`)