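; Level actor that darkens the main level in stages as the boss fight progresses, driven by BP_BossCharacter events bound on BeginPlay.
; Lights50 and Lights5 play timelines scaling directional, sky and two point lights plus local fog extinction, then store the results as the next stage's base.
; LightsOff destroys those lights, the fog and the post-process volume outright; an older timeline fade to zero is left unconnected.
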(event `self.ReceiveBeginPlay`
  (bind _asbp_boss_character (cast `/Game/StarterContent/Blueprints/BP_Boss/BP_BossCharacter` (`self.BossRef`)))
  (add `/Game/StarterContent/Blueprints/BP_Boss/BP_BossCharacter.Lights50` _asbp_boss_character (delegate `Lights50`))
  (add `/Game/StarterContent/Blueprints/BP_Boss/BP_BossCharacter.Lights5` _asbp_boss_character (delegate `Lights5`))
  (add `/Game/StarterContent/Blueprints/BP_Boss/BP_BossCharacter.Lights0` _asbp_boss_character (delegate `LightsOff`)))

(event `Lights50`
  (bind _localfogvolumeref (`self.LocalFogVolumeRef`))
  (`KismetSystemLibrary.PrintString` "Lights 50")
  (bind (_direction _light_value) (`Timeline|Timeline_50`)
    (:`Update`
      (bind _returnvalue (* (`self.DirLightIntensity`) _light_value))
      (`LightComponent.SetIntensity` (`Light.LightComponent` (`self.DirLight`)) _returnvalue)
      (bind _returnvalue_2 (* (`self.SkyLightIntensity`) _light_value))
      (`SkyLightComponent.SetIntensity` (`SkyLight.LightComponent` (`self.SkyLight`)) _returnvalue_2)
      (bind _returnvalue_3 (* (`self.PointLight1Intensity`) _light_value))
      (`LightComponent.SetIntensity` (`PointLight.PointLightComponent` (`self.PointLIght1`)) _returnvalue_3)
      (bind _returnvalue_4 (* (`self.PointLight2Intensity`) _light_value))
      (`LightComponent.SetIntensity` (`PointLight.PointLightComponent` (`self.PointLIght2`)) _returnvalue_4)
      (bind _returnvalue_5 (* (`self.RadialFogDensity`) _light_value))
      (`LocalFogVolumeComponent.SetRadialFogExtinction` (`LocalFogVolume.LocalFogVolumeVolume` _localfogvolumeref) _returnvalue_5)
      (bind _returnvalue_6 (* (`self.HeightFogDensity`) _light_value))
      (`LocalFogVolumeComponent.SetHeightFogExtinction` (`LocalFogVolume.LocalFogVolumeVolume` _localfogvolumeref) _returnvalue_6))
    (:`Finished`
      (set `self.DirLightIntensity` _returnvalue)
      (set `self.SkyLightIntensity` _returnvalue_2)
      (set `self.PointLight1Intensity` _returnvalue_3)
      (set `self.PointLight2Intensity` _returnvalue_4)
      (set `self.RadialFogDensity` _returnvalue_5)
      (set `self.HeightFogDensity` _returnvalue_6))))

(event `Lights5`
  (bind _localfogvolumeref (`self.LocalFogVolumeRef`))
  (`KismetSystemLibrary.PrintString` "LIGHTS5")
  (bind (_direction _light_value) (`Timeline|Timeline_5`)
    (:`Update`
      (bind _returnvalue (* (`self.DirLightIntensity`) _light_value))
      (`LightComponent.SetIntensity` (`Light.LightComponent` (`self.DirLight`)) _returnvalue)
      (bind _returnvalue_2 (* (`self.SkyLightIntensity`) _light_value))
      (`SkyLightComponent.SetIntensity` (`SkyLight.LightComponent` (`self.SkyLight`)) _returnvalue_2)
      (bind _returnvalue_3 (* (`self.PointLight1Intensity`) _light_value))
      (`LightComponent.SetIntensity` (`PointLight.PointLightComponent` (`self.PointLIght1`)) _returnvalue_3)
      (bind _returnvalue_4 (* (`self.PointLight2Intensity`) _light_value))
      (`LightComponent.SetIntensity` (`PointLight.PointLightComponent` (`self.PointLIght2`)) _returnvalue_4)
      (bind _returnvalue_5 (* (`self.RadialFogDensity`) _light_value))
      (`LocalFogVolumeComponent.SetRadialFogExtinction` (`LocalFogVolume.LocalFogVolumeVolume` _localfogvolumeref) _returnvalue_5)
      (bind _returnvalue_6 (* (`self.HeightFogDensity`) _light_value))
      (`LocalFogVolumeComponent.SetHeightFogExtinction` (`LocalFogVolume.LocalFogVolumeVolume` _localfogvolumeref) _returnvalue_6))
    (:`Finished`
      (set `self.DirLightIntensity` _returnvalue)
      (set `self.SkyLightIntensity` _returnvalue_2)
      (set `self.PointLight1Intensity` _returnvalue_3)
      (set `self.PointLight2Intensity` _returnvalue_4)
      (set `self.RadialFogDensity` _returnvalue_5)
      (set `self.HeightFogDensity` _returnvalue_6))))

(event `LightsOff`
  (`KismetSystemLibrary.PrintString` "LIGHTS0")
  (`self.K2_DestroyActor` (`self.DirLight`))
  (`self.K2_DestroyActor` (`self.SkyLight`))
  (`self.K2_DestroyActor` (`self.PostProcessVolume`))
  (`self.K2_DestroyActor` (`self.PointLIght1`))
  (`self.K2_DestroyActor` (`self.PointLIght2`))
  (`self.K2_DestroyActor` (`self.LocalFogVolumeRef`))
  (`KismetSystemLibrary.PrintString` "Main Level Lights Destroyed"))

(fn `UserConstructionScript`)