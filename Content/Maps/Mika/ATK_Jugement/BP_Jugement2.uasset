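; BP_Jugement2 is an actor that drives a radius-based transition effect for a "Jugement" attack through the MPC_Jugement_Transition2 material parameter collection.
; ExpandRadius plays the TL_Jugement timeline and writes its value to the collection's Radius scalar each update, while ShrinkRadius reverses that timeline.
; Nothing in this graph triggers either event.
; A FlipFlop toggle and a BossLoc write from the actor's location are left unconnected.
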(event `self.ReceiveBeginPlay`)

(event `Expand Radius`
  (bind (_direction _radius) (`Timeline|TL_Jugement` :!label _label)
    (:`Update`
      (`KismetMaterialLibrary.SetScalarParameterValue` "/Game/Maps/Mika/ATK_Jugement/MPC_Jugement_Transition2.MPC_Jugement_Transition2" "Radius" _radius))))

(event `Shrink Radius`
  (goto _label :!via `Reverse`))

(event `Key|M`
  (params (Key :type "Key Structure")))

(fn `UserConstructionScript`)