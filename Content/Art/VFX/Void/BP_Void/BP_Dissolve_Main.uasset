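; Dissolve VFX actor that pairs a skeletal mesh's dissolve materials with a Niagara system.
; The construction script runs a setup macro that pushes shared alpha, boosted edge color and dissolve texture to both, creating dynamic material instances per slot.
; A static mesh variant and a timeline animating alpha exist but are disconnected.
; At runtime, only a debug key acts, attaching a sparks emitter to the Head.
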(event Custom|Uptdate%20data%20SK)

(event EventBeginPlay)

(event Collision|EventActorBeginOverlap
  (params (OtherActor :type Actor%20Object%20Reference)))

(event EventTick
  (params (DeltaSeconds :type Float%20%28single-precision%29)))

(event Input|KeyboardEvents|DebugKey1
  (params (Key :type Key%20Structure :default "None") (ActionValue :type Input%20Action%20Value%20Structure))
  (:Pressed
    (Effects|SpawnEmitterAttached "/Game/StarterContent/Particles/P_Sparks.P_Sparks" (Variables|Default|GetSkeletalMesh) "Head")))

(fn ConstructionScript
  (Utilities|SKMeshSetupMacro (Variables|Default|GetSK_Niagara) (Variables|Default|GetSkeletalMesh)))