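; Trigger actor that runs the game's outro cutscene when BP_PlayerSantino first overlaps it.
; It disables player input and plays the LastCinematic level sequence, then runs two timelines from a Sequence node.
; One waits out the sequence's duration, then opens the main menu with cursor and UI-only input.
; The other uses fixed delays to play boss-death and final dialogue cues with data-table-driven subtitle widgets.
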(event `self.ReceiveActorBeginOverlap`
  (params (OtherActor :type "Actor Object Reference"))
  (bind _returnvalue (`GameplayStatics.GetPlayerController` 0))
  (bind _asbp_player_santino (cast `/Game/BP/Characters/BP_PlayerSantino` OtherActor))
  (`/Engine/EditorBlueprintResources/StandardMacros.DoOnce` false
    (:`Completed`
      (`self.DisableInput` _asbp_player_santino null)
      (bind (_outactor _returnvalue_2) (`LevelSequencePlayer.CreateLevelSequencePlayer` "/Game/Cutscene/LastCinematic.LastCinematic"))
      (`MovieSceneSequencePlayer.Play` _returnvalue_2)
      (`|ExecutionSequence`
        (:`then_0`
          (`KismetSystemLibrary.Delay` (`TimeManagementBlueprintLibrary.Conv_QualifiedFrameTimeToSeconds` (`MovieSceneSequencePlayer.GetDuration` _returnvalue_2)))
          (bind _output_get (set `PlayerController.bShowMouseCursor` true _returnvalue))
          (`WidgetBlueprintLibrary.SetInputMode_UIOnlyEx` _returnvalue null "DoNotLock" _output_get)
          (bind _returnvalue_3 (`|CreateWidget` "/Game/UI/WB_MainMenu.WB_MainMenu_C" _returnvalue))
          (`UserWidget.AddToViewport` _returnvalue_3 0))
        (:`then_1`
          (cast `/Game/BP/Characters/BP_PlayerSantino` (`GameplayStatics.GetPlayerCharacter` 0))
          ;[1 0 0.0302 0.502] C8 - BOSS DEAD GG WP
          (`GameplayStatics.SpawnSound2D` "/Game/Maps/Mika/Subtitles/VL_Dialogs/C_8_Cue.C_8_Cue" 1.0 1.0 0.0 null)
          (`KismetSystemLibrary.Delay` 1.0)
          (bind _returnvalue_4 (`|CreateWidget` "/Game/Maps/Mika/Subtitles/UW_Subtitles.UW_Subtitles_C" null (make `DataTableRowHandle` "/Game/Maps/Mika/Subtitles/Voicelines_Subtitiles/DT_Sub_C8.DT_Sub_C8" "1")))
          (`UserWidget.AddToViewport` _returnvalue_4 0)
          (`KismetSystemLibrary.Delay` 20.0)
          ;[1 0.1716 0.821 0.502] MC2 - Final Dialog
          (`GameplayStatics.SpawnSound2D` "/Game/Maps/Mika/Subtitles/VL_Dialogs/MC_2_Cue.MC_2_Cue" 1.0 1.0 0.0 null)
          (`KismetSystemLibrary.PrintString` "mcdialog2")
          (`KismetSystemLibrary.Delay` 1.2)
          (bind _returnvalue_5 (`|CreateWidget` "/Game/Maps/Mika/Subtitles/UW_Subtitles.UW_Subtitles_C" null (make `DataTableRowHandle` "/Game/Maps/Mika/Subtitles/Voicelines_Subtitiles/DT_Sub_MC2.DT_Sub_MC2" "1")))
          (`UserWidget.AddToViewport` _returnvalue_5 0))))))

(fn `UserConstructionScript`)