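; Generic actor pool that pre-spawns a given class and hands out instances for reuse.
; CreatePool spawns hidden actors with collision and tick disabled, and GetActor treats disabled collision as free, then moves and re-enables that actor.
; An exhausted pool grows by one, returning the new actor still disabled and untransformed.
; DesactiveActor affects the pool itself, DesactiveBullet is empty, and GetActor's boss-bullet branch is unreachable.
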(event `CreatePool`
  (params (`Size Pool` :type Integer) (`Actor to Spawn` :type "Actor Class Reference"))
  (set `self.BPActor` `Actor to Spawn`)
  (bind _output_get (set `self.PoolSize` `Size Pool`))
  (for _ (range (+ _output_get 1))
    (bind _returnvalue (`|SpawnActorFromClass` (`self.BPActor`) (`KismetMathLibrary.MakeTransform` (0.0 0.0 0.0)) "Undefined" "MultiplyWithRoot" null null))
    (`self.SetActorHiddenInGame` _returnvalue true)
    (`self.SetActorEnableCollision` _returnvalue false)
    (`self.SetActorTickEnabled` _returnvalue false)
    (`KismetArrayLibrary.Array_Add` (`self.BP_ActeurPool`) _returnvalue)))

(event `Desactive Actor`
  (`self.SetActorHiddenInGame` true)
  (`self.SetActorEnableCollision` false)
  (`self.SetActorTickEnabled` false))

(fn `Create New Pool Size`
  (returns (Actor :type "Actor Object Reference"))
  (`/Engine/EditorBlueprintResources/StandardMacros.IncrementInt` (`self.PoolSize`)
    (:`  `
      (bind _returnvalue (`|SpawnActorFromClass` (`self.BPActor`) (`KismetMathLibrary.MakeTransform` (0.0 0.0 0.0)) "Undefined" "MultiplyWithRoot" null null))
      (`self.SetActorHiddenInGame` _returnvalue true)
      (`self.SetActorEnableCollision` _returnvalue false)
      (`self.SetActorTickEnabled` _returnvalue false)
      (`KismetArrayLibrary.Array_Add` (`self.BP_ActeurPool`) _returnvalue)
      (return _returnvalue))))

(fn `DesactiveBullet`
  (params (Actor :type "Actor Object Reference")))

(fn `GetActor`
  (params (Transform :type "Transform Structure"))
  (returns (bullet :type "Actor Object Reference"))
  (for _array_element (`self.BP_ActeurPool`)
    (if (not (`self.GetActorEnableCollision` _array_element))
      (`self.K2_SetActorTransform` _array_element Transform false false)
      (`self.SetActorHiddenInGame` _array_element false)
      (`self.SetActorEnableCollision` _array_element true)
      (`self.SetActorTickEnabled` _array_element true)
      (return _array_element)))
  (bind _actor (`self.Create New Pool Size`))
  (return _actor))

(fn `switch On actor`
  (params (PoolBulletBoss :type "Array of /Game/ThirdPerson/Blueprints/BP_BulletBoss Object Reference") (transform :type "Transform Structure"))
  (returns (NewParam :type "/Game/ThirdPerson/Blueprints/BP_BulletBoss Object Reference"))
  (for _array_element PoolBulletBoss
    (if (not (`self.GetActorEnableCollision` _array_element))
      (`self.K2_SetActorTransform` _array_element transform false false)
      (`self.SetActorHiddenInGame` _array_element false)
      (`self.SetActorEnableCollision` _array_element true)
      (`self.SetActorTickEnabled` _array_element true)
      (cast `/Game/ThirdPerson/Blueprints/BP_BulletBoss` _array_element)
      (return (stale _asbp_bullet_boss))))
  (bind _actor (`self.Create New Pool Size`))
  (bind _asbp_bullet_boss (cast `/Game/ThirdPerson/Blueprints/BP_BulletBoss` _actor))
  (return _asbp_bullet_boss))

(fn `UserConstructionScript`)