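; Object pool actor that pre-spawns and recycles BP_BulletBoss bullets.
; CreatePool fills the array with bullets that are hidden, with collision and tick disabled; DesactiveBullet returns an actor to that state.
; GetActor and SwitchOnActor treat disabled collision as free to position and re-enable bullets, though GetActor checks the pool's own collision.
; When none qualifies, CreateNewPoolSize grows the pool by one, leaving the new bullet inactive.
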(event `CreatePool`
  (params (`Size Pool` :type Integer))
  (bind _output_get (set `self.PoolSize` `Size Pool`))
  (for _ (range (+ _output_get 1))
    (bind _returnvalue (`|SpawnActorFromClass` "/Game/ThirdPerson/Blueprints/BP_BulletBoss.BP_BulletBoss_C" (`KismetMathLibrary.MakeTransform` (0.0 0.0 0.0)) "Undefined" "MultiplyWithRoot" null null))
    (`self.SetActorHiddenInGame` _returnvalue true)
    (`self.SetActorEnableCollision` _returnvalue false)
    (`self.SetActorTickEnabled` _returnvalue false)
    (`KismetArrayLibrary.Array_Add` (`self.BP_PoolBulletBoss`) _returnvalue)))

(event `Desactive Actor`
  (`self.SetActorHiddenInGame` true)
  (`self.SetActorEnableCollision` false)
  (`self.SetActorTickEnabled` false))

(fn `Create New Pool Size`
  (returns (Actor :type "/Game/ThirdPerson/Blueprints/BP_BulletBoss Object Reference"))
  (`/Engine/EditorBlueprintResources/StandardMacros.IncrementInt` (`self.PoolSize`)
    (:`  `
      (bind _returnvalue (`|SpawnActorFromClass` "/Game/ThirdPerson/Blueprints/BP_BulletBoss.BP_BulletBoss_C" (`KismetMathLibrary.MakeTransform` (0.0 0.0 0.0)) "Undefined" "MultiplyWithRoot" null null))
      (`self.SetActorHiddenInGame` _returnvalue true)
      (`self.SetActorEnableCollision` _returnvalue false)
      (`self.SetActorTickEnabled` _returnvalue false)
      (`KismetArrayLibrary.Array_Add` (`self.BP_PoolBulletBoss`) _returnvalue)
      (return _returnvalue))))

(fn `DesactiveBullet`
  (params (Actor :type "/Game/ThirdPerson/Blueprints/BP_BulletBoss Object Reference"))
  (`self.SetActorHiddenInGame` Actor true)
  (`self.SetActorEnableCollision` Actor false)
  (`self.SetActorTickEnabled` Actor false))

(fn `GetActor`
  (params (Transform :type "Transform Structure"))
  (returns (bullet :type "/Game/ThirdPerson/Blueprints/BP_BulletBoss Object Reference"))
  (for _array_element (`self.BP_PoolBulletBoss`)
    (bind _asbp_bullet_boss (cast `/Game/ThirdPerson/Blueprints/BP_BulletBoss` _array_element))
    (if (not (`self.GetActorEnableCollision`))
      (`self.K2_SetActorTransform` _asbp_bullet_boss Transform false false)
      (`self.SetActorHiddenInGame` _asbp_bullet_boss false)
      (`self.SetActorEnableCollision` _asbp_bullet_boss true)
      (`self.SetActorTickEnabled` _asbp_bullet_boss true)
      (return _asbp_bullet_boss)))
  (bind _actor (`self.Create New Pool Size`))
  (return _actor))

(fn `switch On actor`
  (params (PoolBulletBoss :type "Array of /Game/ThirdPerson/Blueprints/BP_BulletBoss Object Reference") (transform :type "Transform Structure"))
  (returns (NewParam :type "/Game/ThirdPerson/Blueprints/BP_BulletBoss Object Reference"))
  (for _array_element PoolBulletBoss
    (if (not (`self.GetActorEnableCollision` _array_element))
      (`self.K2_SetActorTransform` _array_element transform false false)
      (`self.SetActorHiddenInGame` _array_element false)
      (`self.SetActorEnableCollision` _array_element true)
      (`self.SetActorTickEnabled` _array_element true)
      (cast `/Game/ThirdPerson/Blueprints/BP_BulletBoss` _array_element)
      (return (stale _actor))))
  (bind _actor (`self.Create New Pool Size`))
  (return _actor))

(fn `UserConstructionScript`)