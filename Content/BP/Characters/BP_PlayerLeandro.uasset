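; BP_PlayerLeandro is the player Blueprint, handling shooting, camera shake, camera view switching and HUD creation.
; Normal shots spawn BP_Bullet at a random component tagged ShootSpawns, while charged shots spawn one at every such component.
; A timeline curve scales random camera offsets for shake, triggered by input.
; Another timeline lerps the spring arm's socket offset through preset positions in a cycle; an FOV switch is left unconnected.
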(event `EnhancedInput|/Game/Inputs/Actions/IA_ChargedShoot`
  (params (ActionValue :type Boolean) (ElapsedSeconds :type "Float (double-precision)") (TriggeredSeconds :type "Float (double-precision)") (InputAction :type "InputAction Object Reference" :default "/Game/Inputs/Actions/IA_ChargedShoot.IA_ChargedShoot"))
  (:`Triggered`
    (for _array_element (`self.GetComponentsByTag` "/Script/Engine.StaticMeshComponent" "ShootSpawns")
      (bind (_returnvalue_location _returnvalue_rotation) (`KismetMathLibrary.BreakTransform` (`SceneComponent.K2_GetComponentToWorld` _array_element)))
      (`|SpawnActorFromClass` "/Game/ThirdPerson/Blueprints/BP_Bullet.BP_Bullet_C" (`KismetMathLibrary.MakeTransform` _returnvalue_location _returnvalue_rotation) "AlwaysSpawn" "MultiplyWithRoot" null null))))

(event `EnhancedInput|/Game/Inputs/Actions/IA_Shoot`
  (params (ActionValue :type Boolean) (ElapsedSeconds :type "Float (double-precision)") (TriggeredSeconds :type "Float (double-precision)") (InputAction :type "InputAction Object Reference" :default "/Game/Inputs/Actions/IA_Shoot.IA_Shoot"))
  (bind (_returnvalue_location _returnvalue_rotation) (`KismetMathLibrary.BreakTransform` (`SceneComponent.K2_GetComponentToWorld` (`KismetArrayLibrary.Array_Random` (`self.GetComponentsByTag` "/Script/Engine.StaticMeshComponent" "ShootSpawns")))))
  (:`Triggered`
    (`|SpawnActorFromClass` "/Game/ThirdPerson/Blueprints/BP_Bullet.BP_Bullet_C" (`KismetMathLibrary.MakeTransform` _returnvalue_location _returnvalue_rotation) "AlwaysSpawn" "MultiplyWithRoot" null null)))

(event `CameraShakeHit`
  ; Camera Shake
  (bind (_direction _shakecurve) (`Timeline|TM_CameraShake` :!via `PlayFromStart`)
    (:`Update`
      (set `self.Shake Curve` _shakecurve)
      (bind _output_get (set `self.CameraShakeOffsetX` (* (`self.Shake Curve`) (`KismetMathLibrary.RandomFloatInRange` (`self.ShakeIntensityMin`) (`self.ShakeIntensityMax`)))))
      (bind _output_get_2 (set `self.CameraShakeOffsetY` (* (`self.Shake Curve`) (`KismetMathLibrary.RandomFloatInRange` (`self.ShakeIntensityMin`) (`self.ShakeIntensityMax`)))))
      (bind _output_get_3 (set `self.CameraShakeOffsetZ` (* (`self.Shake Curve`) (`KismetMathLibrary.RandomFloatInRange` (`self.ShakeIntensityMin`) (`self.ShakeIntensityMax`)))))
      (`SceneComponent.K2_SetRelativeLocation` (`self.Camera`) (`KismetMathLibrary.MakeVector` _output_get _output_get_2 _output_get_3) false false))
    (:`Finished`
      (`SceneComponent.K2_SetRelativeLocation` (`self.Camera`) (0.0 0.0 0.0) false false))))

(event `EnhancedInput|/Game/Inputs/Actions/IA_CameraShake`
  (params (ActionValue :type Boolean) (ElapsedSeconds :type "Float (double-precision)") (TriggeredSeconds :type "Float (double-precision)") (InputAction :type "InputAction Object Reference" :default "/Game/Inputs/Actions/IA_CameraShake.IA_CameraShake"))
  ; Camera Shake
  (:`Triggered`
    (`self.CameraShakeHit` :!label _label)))

(event `Key|F`
  (params (Key :type "Key Structure"))
  ; Camera Shake
  (:`Pressed`
    (goto _label)))

(event `self.ReceiveBeginPlay`
  (bind _camerapositions (`self.CameraPositions`))
  ; Add cam to array
  (`KismetArrayLibrary.Array_Add` _camerapositions (0.0 20.0 20.0))
  (`KismetArrayLibrary.Array_Add` _camerapositions (153.0 1.0 17.0))
  (`KismetArrayLibrary.Array_Add` _camerapositions (300.0 15.0 -7.0))
  (bind _returnvalue (`|CreateWidget` "/Game/UI/WB_HUD.WB_HUD_C"))
  (`UserWidget.AddToViewport` _returnvalue 0))

(event `CameraChange`
  ; Camera Change
  (bind _result (`/Engine/EditorBlueprintResources/StandardMacros.IncrementInt` (`self.ChangeIndexCam`))
    (:`  `
      (if (< _result (`KismetArrayLibrary.Array_Length` (`self.CameraPositions`)))
        (bind (_direction _camerachange) (`Timeline|TM_CameraChange` :!via `PlayFromStart` :!label _label_2)
          (:`Update`
            (set `SpringArmComponent.SocketOffset` (`KismetMathLibrary.VLerp` (`SpringArmComponent.SocketOffset` (`self.SpringArm`)) (`|GetArrayItem` (`self.CameraPositions`) (`self.ChangeIndexCam`)) _camerachange) (`self.SpringArm`))))
        (else
          (set `self.ChangeIndexCam` 0)
          (goto _label_2 :!via `PlayFromStart`))))))

(event `EnhancedInput|/Game/Inputs/Actions/IA_CameraChange`
  (params (ActionValue :type Boolean) (ElapsedSeconds :type "Float (double-precision)") (TriggeredSeconds :type "Float (double-precision)") (InputAction :type "InputAction Object Reference" :default "/Game/Inputs/Actions/IA_CameraChange.IA_CameraChange"))
  ; Camera Change
  (:`Completed`
    (`self.CameraChange`)))

(fn `UserConstructionScript`)