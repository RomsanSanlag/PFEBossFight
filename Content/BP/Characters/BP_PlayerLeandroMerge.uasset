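; Leandro player character for a boss fight, handling shooting, hit blinking, lasers that damage the boss, death restarts and pause.
; Camera transitions lerp the spring arm socket offset using per-transition curves and durations, alongside triggered shakes.
; A delay chain plays intro voice lines with subtitles; holding X fills a slider that skips the cinematic and enables HUD and shooting.
; Niagara lifetime follows movement, and W starts timed shadow spawning.
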(event `self.ReceiveTick`
  (params (DeltaSeconds :type "Float (single-precision)"))
  (bind _blinkdelay (`self.BlinkDelay`))
  ; Blinking on hit
  (if (and (`self.isInvincible`) (!= (`self.IsDodging`) true))
    (bind _output_get (set `self.Time` (+ DeltaSeconds (`self.Time`))))
    (if (< (mod _output_get (* _blinkdelay 2.0)) _blinkdelay)
      (`PrimitiveComponent.SetMaterial` (`self.Mesh`) 0 (`self.Material Hit`))
      (else
        (`PrimitiveComponent.SetMaterial` (`self.Mesh`) 0 (`self.Material normal`) :!label _label)))
    (else
      (goto _label)))
  (if (== (`self.GetVelocity`) (`KismetMathLibrary.MakeVector` 0.0))
    (`NiagaraComponent.SetVariableFloat` (`self.Niagara`) "LifeTime" (`KismetMathLibrary.RandomFloatInRange` 0.5 0.7))
    (else
      (`NiagaraComponent.SetVariableFloat` (`self.Niagara`) "LifeTime" (`KismetMathLibrary.RandomFloatInRange` 0.1 0.15)))))

(event `EnhancedInput|/Game/Inputs/Actions/IA_Shoot`
  (params (ActionValue :type Boolean) (ElapsedSeconds :type "Float (double-precision)") (TriggeredSeconds :type "Float (double-precision)") (InputAction :type "InputAction Object Reference" :default "/Game/Inputs/Actions/IA_Shoot.IA_Shoot"))
  (bind (_returnvalue_location _returnvalue_rotation) (`KismetMathLibrary.BreakTransform` (`SceneComponent.K2_GetComponentToWorld` (`KismetArrayLibrary.Array_Random` (`self.GetComponentsByTag` "/Script/Engine.StaticMeshComponent" "ShootSpawns")))))
  (:`Triggered`
    (if (`/Game/UI/WB_MainMenuMIKA.CanShoot` (`self.WP MainMenuMika Ref`))
      (if (not (`self.IsShooting`))
        (`|SpawnActorFromClass` "/Game/ThirdPerson/Blueprints/BP_BulletLeandro.BP_BulletLeandro_C" (`KismetMathLibrary.MakeTransform` _returnvalue_location _returnvalue_rotation) "AlwaysSpawn" "MultiplyWithRoot" null null)
        (set `self.IsShooting` true)
        (`KismetSystemLibrary.Delay` (`self.CD Bullet`))
        (set `self.IsShooting` false)))))

(event `EnhancedInput|/Game/Inputs/Actions/IA_Dodge`
  (params (ActionValue :type Boolean) (ElapsedSeconds :type "Float (double-precision)") (TriggeredSeconds :type "Float (double-precision)") (InputAction :type "InputAction Object Reference" :default "/Game/Inputs/Actions/IA_Dodge.IA_Dodge")))

(event `self.ReceiveBeginPlay`
  (bind _camerapositions (`self.CameraPositions`))
  ; J'ai besoin de call un truc au debut du jeu, si vous savez comment faire en plus clean go me le dire svp (mika)
  (`|ExecutionSequence`
    (:`then_0`
      ; Add cam to array
      (`KismetArrayLibrary.Array_Add` _camerapositions (0.0 20.0 20.0))
      (`KismetArrayLibrary.Array_Add` _camerapositions (153.0 1.0 17.0))
      (`KismetArrayLibrary.Array_Add` _camerapositions (300.0 15.0 -7.0)))
    (:`then_1`
      ; Skip Input pour l'intro (MIKA)
      (`|ExecutionSequence`
        (:`then_0`
          (`KismetSystemLibrary.PrintString` "ref success"))
        (:`then_1`
          (if (>= (`self.SubsSKIP(MIKA)`) (`KismetStringLibrary.Conv_StringToDouble` "1")) :!label _label_2
            (`/Engine/EditorBlueprintResources/StandardMacros.DoOnce` false
              (:`Completed`
                ;[1 1 1] DIALOGUE D'INTRODUCTION
                ;;[1 0.7871 0 0.5] C1.1 - BOSS FIRST LINE
                (bind _returnvalue (`GameplayStatics.SpawnSound2D` "/Game/Maps/Mika/Subtitles/VL_Dialogs/C_1_1_Cue.C_1_1_Cue" 1.0 1.0 0.0 null))
                (bind _output_get (set `self.SubRef(MIKA)` _returnvalue))
                (`KismetSystemLibrary.Delay` 0.5)
                (bind _returnvalue_2 (`|CreateWidget` "/Game/Maps/Mika/Subtitles/UW_Subtitles.UW_Subtitles_C" null (make `DataTableRowHandle` "/Game/Maps/Mika/Subtitles/Voicelines_Subtitiles/DT_Sub.DT_Sub" "1")))
                (bind _output_get_2 (set `self.W_SubRef(MIKA)` _returnvalue_2))
                (`UserWidget.AddToViewport` _output_get_2 0)
                (`KismetSystemLibrary.Delay` 13.0)
                (if (> (`AudioComponent.VolumeMultiplier` _output_get) (`KismetStringLibrary.Conv_StringToDouble` "0"))
                  (`/Engine/EditorBlueprintResources/StandardMacros.IsValid` _output_get
                    (:`Is Valid`
                      ;;[1 0.07963 0.9859 0.5] MC1 - PLAYER
                      (bind _returnvalue_3 (`GameplayStatics.SpawnSound2D` "/Game/Maps/Mika/Subtitles/VL_Dialogs/MC_1_Cue.MC_1_Cue" 1.0 1.0 0.0 null))
                      (bind _output_get_3 (set `self.SubRef2(MIKA)` _returnvalue_3))
                      (`KismetSystemLibrary.Delay` 1.25)
                      (bind _returnvalue_4 (`|CreateWidget` "/Game/Maps/Mika/Subtitles/UW_Subtitles.UW_Subtitles_C" null (make `DataTableRowHandle` "/Game/Maps/Mika/Subtitles/Voicelines_Subtitiles/DT_Sub_MC1.DT_Sub_MC1" "1")))
                      (bind _output_get_4 (set `self.W_SubRef2(MIKA)` _returnvalue_4))
                      (`UserWidget.AddToViewport` _output_get_4 0)
                      (`KismetSystemLibrary.Delay` 18.0)
                      ;;[1 0.7882 0 0.502] C1.2 - BOSS
                      (bind _returnvalue_5 (`GameplayStatics.SpawnSound2D` "/Game/Maps/Mika/Subtitles/VL_Dialogs/C_1_2_Cue.C_1_2_Cue" 1.0 1.0 0.0 null))
                      (set `self.SubRef3(MIKA)` _returnvalue_5)
                      (`KismetSystemLibrary.Delay` 0.7)
                      (bind _returnvalue_6 (`|CreateWidget` "/Game/Maps/Mika/Subtitles/UW_Subtitles.UW_Subtitles_C" null (make `DataTableRowHandle` "/Game/Maps/Mika/Subtitles/Voicelines_Subtitiles/DT_Sub_C1-2.DT_Sub_C1-2" "1")))
                      (bind _output_get_5 (set `self.W_SubRef3(MIKA)` _returnvalue_6))
                      (`UserWidget.AddToViewport` _output_get_5 0)
                      (`KismetSystemLibrary.Delay` 9.0)
                      (`Widget.RemoveFromParent` (`self.WB Skip Ref`))
                      (set `/Game/UI/WB_MainMenuMIKA.canPause` true (`self.WP MainMenuMika Ref`)))))))
            (elif (== (`self.SubsSKIP(MIKA)`) (`KismetStringLibrary.Conv_StringToDouble` "0"))
              (`KismetSystemLibrary.Delay` 1.0)
              (goto _label_2))))
        (:`then_2`
          (bind _foundwidgets (`WidgetBlueprintLibrary.GetAllWidgetsOfClass` null)))))))

(event `Key|W`
  (params (Key :type "Key Structure"))
  (:`Pressed`
    (`KismetSystemLibrary.K2_SetTimerDelegate` (delegate `CustomEvent`) 0.05 true))
  (:`Released`
    (`KismetSystemLibrary.K2_PauseTimer` null "CustomEvent")
    (`ActorComponent.Deactivate` (`self.Niagara1`))))

(event `self.OnCameraTransition`
  (params (indexToGo :type Integer))
  (bind (_foundtransition_fromindex _foundtransition_toindex _foundtransition_duration _foundtransition_curve) (break `/Game/BP/Camera/Transitions/ST_CameraTransition` (`self.FoundTransition`)))
  (bind _currentcurve (`self.CurrentCurve`))
  ; Camera Transitions Manager
  (set `self.OldIndex` (`self.CurrentCameraIndex`))
  (bind _output_get (set `self.CurrentCameraIndex` indexToGo))
  (set `self.StartSocket` (`SpringArmComponent.SocketOffset` (`self.SpringArm`)))
  (set `self.TargetSocket` (`|GetArrayItem` (`self.CameraPositions`) _output_get))
  (for _array_element (`self.Transitions`)
    (bind (_fromindex _toindex) (break `/Game/BP/Camera/Transitions/ST_CameraTransition` _array_element))
    (if (and (== (`self.OldIndex`) _fromindex) (== _toindex (`self.CurrentCameraIndex`)))
      (set `self.FoundTransition` _array_element)))
  (bind _output_get_2 (set `self.CurrentDuration` _foundtransition_duration))
  (set `self.CurrentCurve` _foundtransition_curve)
  (`TimelineComponent.SetPlayRate` (`self.TMCameraTransition`) (/ 1.0 _output_get_2))
  (bind (_direction _alpha) (`Timeline|TMCameraTransition` :!via `PlayFromStart`)
    (:`Update`
      (`/Engine/EditorBlueprintResources/StandardMacros.IsValid` _currentcurve
        (:`Is Valid`
          (set `SpringArmComponent.SocketOffset` (`KismetMathLibrary.VLerp` (`self.StartSocket`) (`self.TargetSocket`) (`CurveFloat.GetFloatValue` _currentcurve _alpha)) (`self.SpringArm`)))))))

(event `CustomEvent`
  (`|SpawnActorFromClass` "/Game/VFX/VFX/Void/BP_Void/BP_Shadow.BP_Shadow_C" (`SceneComponent.K2_GetComponentToWorld` (`self.Mesh`)) "Undefined" "MultiplyWithRoot" null null)
  (`ActorComponent.Activate` (`self.Niagara1`) true))

(event `self.OnDomagePlayer`
  (params (PV :type Integer))
  (if (and (== PV 0) (`self.WantToDie`))
    (bind _returnvalue (`GameplayStatics.GetCurrentLevelName` true))
    (`GameplayStatics.OpenLevel` (`KismetStringLibrary.Conv_StringToName` _returnvalue))
    (else
      (`self.SetInvicibleAfterHit`))))

(event `EnhancedInput|/Game/Inputs/Actions/IA_CameraChange`
  (params (ActionValue :type Boolean) (ElapsedSeconds :type "Float (double-precision)") (TriggeredSeconds :type "Float (double-precision)") (InputAction :type "InputAction Object Reference" :default "/Game/Inputs/Actions/IA_CameraChange.IA_CameraChange")))

(event `self.OnCameraShake`
  (params (isSlowShake :type Boolean) (intensity :type "Float (single-precision)"))
  (bind _camerashakesource (`self.CameraShakeSource`))
  (bind _output (`|GetArrayItem` (`self.Shakes`) 1))
  (if isSlowShake
    (bind (_direction _intensity) (`Timeline|Timeline_0` :!via `PlayFromStart`)
      (:`Update`
        (`CameraShakeSourceComponent.StartCameraShake` :`self` _camerashakesource :`InCameraShake` _output :`Scale` _intensity)))
    (else
      (`CameraShakeSourceComponent.StartCameraShake` :`self` _camerashakesource :`InCameraShake` _output :`Scale` intensity))))

(event `EnhancedInput|/Game/Inputs/Actions/IA_CameraShake`
  (params (ActionValue :type Boolean) (ElapsedSeconds :type "Float (double-precision)") (TriggeredSeconds :type "Float (double-precision)") (InputAction :type "InputAction Object Reference" :default "/Game/Inputs/Actions/IA_CameraShake.IA_CameraShake")))

(event `self.OnLaserLaunched`
  (params (OtherActor :type "Actor Object Reference"))
  (bind _asbp_boss_character (cast `/Game/StarterContent/Blueprints/BP_Boss/BP_BossCharacter` OtherActor))
  (`/Game/StarterContent/Blueprints/BP_Boss/BP_BossCharacter.GetHit` _asbp_boss_character 20))

(event `EnhancedInput|/Game/Maps/Mika/Skip/IA_Skip`
  (params (ActionValue :type Boolean) (ElapsedSeconds :type "Float (double-precision)") (TriggeredSeconds :type "Float (double-precision)") (InputAction :type "InputAction Object Reference" :default "/Game/Maps/Mika/Skip/IA_Skip.IA_Skip"))
  ; Skip Input pour l'intro (MIKA)
)

(event `Key|X`
  (params (Key :type "Key Structure"))
  (bind _wb_skip_ref (`self.WB Skip Ref`))
  (bind _wp_mainmenumika_ref (`self.WP MainMenuMika Ref`))
  (bind _introcinematicref_mika_ (`self.IntroCinematicRef(MIKA)`))
  (bind _wb_skip_ref_2 (`self.WB Skip Ref`))
  (bind _subref_mika_ (`self.SubRef(MIKA)`))
  (bind _subref2_mika_ (`self.SubRef2(MIKA)`))
  (bind _subref3_mika_ (`self.SubRef3(MIKA)`))
  ; Skip Input pour l'intro (MIKA)
  (:`Pressed`
    (`|ExecutionSequence`
      (:`then_0`
        (`/Engine/EditorBlueprintResources/StandardMacros.DoOnce` false
          (:`Completed`
            (`WidgetBlueprintLibrary.GetAllWidgetsOfClass` "/Game/Maps/Mika/Skip/WBP_Skip.WBP_Skip_C")
            (`WidgetBlueprintLibrary.GetAllWidgetsOfClass` "/Game/Maps/Mika/Subtitles/UW_Subtitles.UW_Subtitles_C"))))
      (:`then_1`
        (if (not (`/Game/UI/WB_MainMenuMIKA.IsInMainMenu?` (`self.WP MainMenuMika Ref`)))
          (`/Engine/EditorBlueprintResources/StandardMacros.IsValid` _wb_skip_ref_2
            (:`Is Valid`
              (if (`Widget.IsInViewport` _wb_skip_ref_2)
                (bind (_direction _skipslider) (`Timeline|Timeline` :!label _label_3)
                  (:`Update`
                    (`/Engine/EditorBlueprintResources/StandardMacros.IsValid` _wb_skip_ref
                      (:`Is Valid`
                        (`/Game/Maps/Mika/Skip/WBP_Skip.UpdateSkipSlider` _wb_skip_ref _skipslider))))
                  (:`Finished`
                    (if (== _skipslider (`KismetStringLibrary.Conv_StringToDouble` "1"))
                      (`/Engine/EditorBlueprintResources/StandardMacros.DoOnce` false
                        (:`Completed`
                          (`|ExecutionSequence`
                            (:`then_0`
                              (`Widget.RemoveFromParent` (`self.WB Skip Ref`))
                              (`KismetSystemLibrary.PrintString` "REMOVE")
                              (set `/Game/UI/WB_MainMenuMIKA.CanShoot` true _wp_mainmenumika_ref)
                              (set `/Game/UI/WB_MainMenuMIKA.canPause` true _wp_mainmenumika_ref)
                              (bind _returnvalue (`|CreateWidget` "/Game/UI/WB_HUD.WB_HUD_C"))
                              (`UserWidget.AddToViewport` _returnvalue 0))
                            (:`then_1`
                              (`/Engine/EditorBlueprintResources/StandardMacros.IsValid` _introcinematicref_mika_
                                (:`Is Valid`
                                  (`|ExecutionSequence`
                                    (:`then_0`
                                      (`MovieSceneSequencePlayer.GoToEndAndStop` _introcinematicref_mika_)
                                      (bind _returnvalue_2 (`GameplayStatics.GetActorOfClass` "/Script/Engine.CameraActor"))
                                      (`self.K2_DestroyActor` _returnvalue_2)
                                      (`WidgetBlueprintLibrary.SetInputMode_GameOnly` (`GameplayStatics.GetPlayerController` 0))
                                      (bind _foundwidgets (`WidgetBlueprintLibrary.GetAllWidgetsOfClass` "/Game/UI/WB_HUD.WB_HUD_C" false))
                                      (`Widget.SetVisibility` _foundwidgets "Visible"))
                                    (:`then_1`
                                      (`/Engine/EditorBlueprintResources/StandardMacros.IsValid` _subref_mika_
                                        (:`Is Valid`
                                          (`AudioComponent.FadeOut` _subref_mika_ 0.5 0.0 "Linear")
                                          (`Widget.RemoveFromParent` (`self.W_SubRef(MIKA)`)))))
                                    (:`then_2`
                                      (`/Engine/EditorBlueprintResources/StandardMacros.IsValid` _subref2_mika_
                                        (:`Is Valid`
                                          (`AudioComponent.FadeOut` _subref2_mika_ 0.5 0.0 "Linear")
                                          (`Widget.RemoveFromParent` (`self.W_SubRef2(MIKA)`)))))
                                    (:`then_3`
                                      (`/Engine/EditorBlueprintResources/StandardMacros.IsValid` _subref3_mika_
                                        (:`Is Valid`
                                          (`AudioComponent.FadeOut` _subref3_mika_ 0.5 0.0 "Linear")
                                          (`Widget.RemoveFromParent` (`self.W_SubRef3(MIKA)`))))))))))))))))))))))
  (:`Released`
    (goto _label_3 :!via `Reverse`)))

(event `EnhancedInput|/Game/Inputs/Actions/IA_Pause`
  (params (ActionValue :type Boolean) (ElapsedSeconds :type "Float (double-precision)") (TriggeredSeconds :type "Float (double-precision)") (InputAction :type "InputAction Object Reference" :default "/Game/Inputs/Actions/IA_Pause.IA_Pause"))
  (bind _returnvalue (`GameplayStatics.GetPlayerController` 0))
  (bind _returnvalue_2 (`GameplayStatics.GetPlayerController` 0))
  (bind _wbp_pausemika (`self.WBP_PauseMIKA`))
  (:`Started`
    (if (`/Game/UI/WB_MainMenuMIKA.canPause` (`self.WP MainMenuMika Ref`))
      (`/Engine/EditorBlueprintResources/StandardMacros.IsValid` (`self.WBP_PauseMIKA`)
        (:`Is Valid`
          _)
        (:`Is Not Valid`
          (bind _returnvalue_3 (`|CreateWidget` "/Game/UI/WB_PauseMenu.WB_PauseMenu_C"))
          (set `self.WBP_PauseMIKA` _returnvalue_3)))
      (if (`GameplayStatics.IsGamePaused`)
        (`Widget.RemoveFromParent` _wbp_pausemika)
        (`GameplayStatics.SetGamePaused` false)
        (set `PlayerController.bShowMouseCursor` false _returnvalue_2)
        (`WidgetBlueprintLibrary.SetInputMode_GameOnly` _returnvalue_2)
        (else
          (`UserWidget.AddToViewport` _wbp_pausemika 0)
          (`GameplayStatics.SetGamePaused` true)
          (set `PlayerController.bShowMouseCursor` true _returnvalue)
          (`WidgetBlueprintLibrary.SetInputMode_GameAndUIEx` _returnvalue null))))))

(fn `UserConstructionScript`)