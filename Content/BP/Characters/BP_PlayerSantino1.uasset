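; Player character Blueprint that handles shooting, camera effects and HUD creation.
; Tick polls the shoot input, spawning bullets along the camera rotation with a cooldown delay that loops while held.
; Timelines lerp the spring arm back to its default offset and randomly shake the camera; preset cycling is unwired, and Perfect/HeavyShot camera events are empty.
; Holding W runs a timer that spawns BP_Shadow copies at the mesh transform.
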(event `self.ReceiveTick`
  (params (DeltaSeconds :type "Float (single-precision)"))
  (if (`|GetInputActionValue`)
    (set `self.IsPressed` true)
    (if (and (`self.IsPressed`) (`self.CanShoot`)) :!label _label
      (`|SpawnActorFromClass` "/Game/ThirdPerson/Blueprints/BP_Bullet.BP_Bullet_C" (`KismetMathLibrary.MakeTransform` (`SceneComponent.K2_GetComponentLocation` (`self.SpawnBullet`)) (`SceneComponent.K2_GetComponentRotation` (`self.Camera`))) "AlwaysSpawn" "MultiplyWithRoot" null null)
      (set `self.CanShoot` false)
      (`KismetSystemLibrary.Delay` (`self.CD Bullet`))
      (set `self.CanShoot` true)
      (goto _label))
    (else
      (set `self.IsPressed` false))))

(event `ToCameraDefault`
  (params (IsFromHeavyCamera :type Boolean :default false))
  (bind (_direction _movefromperfect _movefromheavy) (`Timeline|TM_ToCameraDefault` :!via `PlayFromStart`)
    (:`Update`
      (if IsFromHeavyCamera
        (set `SpringArmComponent.SocketOffset` (`KismetMathLibrary.VLerp` (`SpringArmComponent.SocketOffset` (`self.SpringArm`)) (`|GetArrayItem` (`self.CameraPositions`)) _movefromheavy) (`self.SpringArm`))
        (else
          ; Effect Perfect To Default
          (set `SpringArmComponent.SocketOffset` (`KismetMathLibrary.VLerp` (`SpringArmComponent.SocketOffset` (`self.SpringArm`)) (`|GetArrayItem` (`self.CameraPositions`)) _movefromperfect) (`self.SpringArm`)))))))

(event `CameraShakeHit`
  ; Camera Shake
  (bind (_direction _shakecurve) (`Timeline|TM_CameraShake` :!via `PlayFromStart`)
    (:`Update`
      (set `self.Shake Curve` _shakecurve)
      (bind _output_get (set `self.CameraShakeOffsetX` (* (`self.Shake Curve`) (`KismetMathLibrary.RandomFloatInRange` (`self.ShakeIntensityMin`) (`self.ShakeIntensityMax`)))))
      (bind _output_get_2 (set `self.CameraShakeOffsetY` (* (`self.Shake Curve`) (`KismetMathLibrary.RandomFloatInRange` (`self.ShakeIntensityMin`) (`self.ShakeIntensityMax`)))))
      (bind _output_get_3 (set `self.CameraShakeOffsetZ` (* (`self.Shake Curve`) (`KismetMathLibrary.RandomFloatInRange` (`self.ShakeIntensityMin`) (`self.ShakeIntensityMax`)))))
      (`SceneComponent.K2_SetRelativeLocation` (`self.Camera`) (`KismetMathLibrary.MakeVector` _output_get _output_get_2 _output_get_3) false false))
    (:`Finished`
      (`SceneComponent.K2_SetRelativeLocation` (`self.Camera`) (0.0 0.0 0.0) false false))))

(event `EnhancedInput|/Game/Inputs/Actions/IA_CameraShake`
  (params (ActionValue :type Boolean) (ElapsedSeconds :type "Float (double-precision)") (TriggeredSeconds :type "Float (double-precision)") (InputAction :type "InputAction Object Reference" :default "/Game/Inputs/Actions/IA_CameraShake.IA_CameraShake"))
  ; Camera Shake
  (:`Triggered`
    (`self.CameraShakeHit` :!label _label_2)))

(event `EnhancedInput|/Game/Inputs/Actions/IA_CameraChange`
  (params (ActionValue :type Boolean) (ElapsedSeconds :type "Float (double-precision)") (TriggeredSeconds :type "Float (double-precision)") (InputAction :type "InputAction Object Reference" :default "/Game/Inputs/Actions/IA_CameraChange.IA_CameraChange"))
  (:`Started`
    (`self.ToCameraDefault` true)))

(event `Key|F`
  (params (Key :type "Key Structure"))
  ; Camera Shake
  (:`Pressed`
    (goto _label_2)))

(event `ToCameraPerfect`)

(event `ToCameraHeavyShot`)

(event `self.ReceiveBeginPlay`
  (bind _camerapositions (`self.CameraPositions`))
  ; Add cam to array
  (`KismetArrayLibrary.Array_Add` _camerapositions (0.0 20.0 20.0))
  (`KismetArrayLibrary.Array_Add` _camerapositions (153.0 1.0 17.0))
  (`KismetArrayLibrary.Array_Add` _camerapositions (300.0 15.0 -7.0))
  (bind _returnvalue (`|CreateWidget` "/Game/UI/WB_HUD.WB_HUD_C"))
  (`UserWidget.AddToViewport` _returnvalue 0))

(event `CameraChange`
  ; Camera Change
  (bind _result (`/Engine/EditorBlueprintResources/StandardMacros.IncrementInt` (`self.ChangeIndexCam`))
    (:`  `
      (if (< _result (`KismetArrayLibrary.Array_Length` (`self.CameraPositions`)))
        (bind (_direction _camerachange) (`Timeline|TM_CameraChange` :!via `PlayFromStart` :!label _label_3)
          (:`Update`
            (set `SpringArmComponent.SocketOffset` (`KismetMathLibrary.VLerp` (`SpringArmComponent.SocketOffset` (`self.SpringArm`)) (`|GetArrayItem` (`self.CameraPositions`) (`self.ChangeIndexCam`)) _camerachange) (`self.SpringArm`))))
        (else
          (set `self.ChangeIndexCam` 0)
          (goto _label_3 :!via `PlayFromStart`))))))

(event `Key|W`
  (params (Key :type "Key Structure"))
  (:`Pressed`
    (`KismetSystemLibrary.K2_SetTimerDelegate` (delegate `CustomEvent`) 0.05 true))
  (:`Released`
    (`KismetSystemLibrary.K2_PauseTimer` null "CustomEvent")))

(event `CustomEvent`
  (`|SpawnActorFromClass` "/Game/VFX/VFX/Void/BP_Void/BP_Shadow.BP_Shadow_C" (`SceneComponent.K2_GetComponentToWorld` (`self.Mesh`)) "Undefined" "MultiplyWithRoot" null null)
  (`KismetSystemLibrary.PrintString` "Hello"))

(fn `UserConstructionScript`)