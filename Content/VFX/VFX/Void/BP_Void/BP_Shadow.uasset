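; BP_Shadow is a short-lived afterimage actor that leaves a frozen copy of the player character, apparently for a dash effect.
; On BeginPlay its poseable mesh takes the player's skeletal mesh, copies the current pose once and swaps in the M_Dash_Perfect material with a random scalar parameter.
; A timeline then drives the material's Alpha parameter, and the actor destroys itself when the timeline finishes.
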(event `self.ReceiveBeginPlay`
  (bind _poseablemesh (`self.PoseableMesh`))
  (bind _poseablemesh_2 (`self.PoseableMesh`))
  (bind _mesh (`Character.Mesh` (`GameplayStatics.GetPlayerCharacter` 0)))
  (`SkinnedMeshComponent.SetSkinnedAssetAndUpdate` _poseablemesh (`SkeletalMeshComponent.SkeletalMeshAsset` _mesh) true)
  (`PrimitiveComponent.SetMaterial` _poseablemesh 0 "/Game/VFX/VFX/Void/Materials/M_Dash_Perfect.M_Dash_Perfect")
  (`PrimitiveComponent.SetMaterial` _poseablemesh 1 "/Game/VFX/VFX/Void/Materials/M_Dash_Perfect.M_Dash_Perfect")
  (`MeshComponent.SetScalarParameterValueOnMaterials` _poseablemesh_2 "Random" (`KismetMathLibrary.RandomFloat`))
  (`PoseableMeshComponent.CopyPoseFromSkeletalComponent` _poseablemesh_2 _mesh)
  (bind (_direction _newtrack_0) (`Timeline|Timeline` :!via `PlayFromStart`)
    (:`Update`
      (`MeshComponent.SetScalarParameterValueOnMaterials` _poseablemesh_2 "Alpha" _newtrack_0))
    (:`Finished`
      (`self.K2_DestroyActor`))))

(fn `UserConstructionScript`)